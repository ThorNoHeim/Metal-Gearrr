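; Damage system Blueprint component that manages an actor's health, healing, blocking and death.
; ActorTakeDamage runs a damage info struct through CanBeDamaged, which routes to blocked, damage or no damage based on death, invincibility and block state.
; Results fire OnBlocked with parry eligibility, OnDeath at zero health, or OnDamageResponse when the actor is interruptible or interruption is forced.
; HealActor adds clamped health to living actors only.
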(event EventBeginPlay)

(event EventTick
  (params (DeltaSeconds :type Float%20%28single-precision%29)))

(fn HealActor
  (params (HealAmount :type Float%20%28double-precision%29))
  (if (not (Variables|Default|GetisDead?))
    (bind _output_get (Variables|Default|SetActorCurrentHealth (Math|Float|Clamp(Float) (+ HealAmount (Variables|Default|GetActorCurrentHealth)) 0.0 (Variables|Default|GetActorMaxHealth))))
    (return _output_get)))

(fn ActorTakeDamage
  (params (DamageInfo :type S%20Damage%20Info%20Structure))
  (bind (_damageamount _damagetype _damageresponse _shoulddamageinvincible _canbeblocked _canbeparried _shouldforceinterupt) (Utilities|Struct|BreakS_DamageInfo DamageInfo))
  (Utilities|CanbeDamaged _shoulddamageinvincible _canbeblocked
    (:DamageBlocked?
      (Default|CallOnBlocked _canbeparried)
      (return false))
    (:TakeDamage?
      (bind _output_get (Variables|Default|SetActorCurrentHealth (- (Variables|Default|GetActorCurrentHealth) _damageamount)))
      (if (<= _output_get 0.0)
        (Variables|Default|SetisDead? true)
        (Default|CallOnDeath)
        (return true)
        (elif (or (Variables|Default|Getinteruptible?) _shouldforceinterupt)
          (Default|CallOnDamageResponse _damageresponse)
          (return true))))
    (:TakeNoDamage?
      (return false))))