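; Ranged soldier enemy that spawns a rifle on BeginPlay and attaches it to its right-hand socket.
; Attack plays a fire montage whose notify line-traces from the weapon to the AI controller's attack target; a second trace runs only if the first finds no hit, sending damage to any hit actor.
; It supplies attack and circling ranges and forwards health queries and healing to BPCDamageSystem, while its own ActorTakeDamage just returns false.
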(event EventBeginPlay
  (CallFunction|EquipWeapon))

(event EventEquipWeapon
  (bind _returnvalue (Game|SpawnActorfromClass "/Game/Characters/Enemies/Enemy_Soldier/Weapons/BP_WeaponRifle.BP_WeaponRifle_C" (Math|Transform|MakeTransform "0, 0, 0") "Undefined" "MultiplyWithRoot" 0 0))
  (bind _output_get (Variables|Default|SetWeaponActor _returnvalue))
  (Transformation|AttachComponentToComponent _output_get (Variables|Character|GetMesh) "RightHand_Rifle_socket" "SnapToTarget" "SnapToTarget" "SnapToTarget" true)
  (Variables|Default|SetisWieldingWeapon true)
  (Default|CallOnWieldWeapon))

(event EventAttack
  (bind _weaponactor (Variables|Default|GetWeaponActor))
  (bind _returnvalue (Transformation|GetActorLocation _weaponactor))
  (bind _notifyname (Animation|Montage|PlayMontage (Variables|Character|GetMesh) "/Game/Characters/Enemies/Enemy_Soldier/enemySoldier_Animations/AM_Fire_SemiAuto_Idle_Montage.AM_Fire_SemiAuto_Idle_Montage")
    (:OnCompleted
      (Default|CallOnAttackEnd :!label _label))
    (:OnInterrupted
      (goto _label))
    (:OnNotifyBegin
      (switch name _notifyname
        (:Fire
          (bind _asaic_enemy_base_aicontroller (Utilities|Casting|CastToAIC_enemyBase_AIController (AI|GetAIController self)))
          (bind _attack_target (Variables|/Game/Characters/Enemies/Enemy_Soldier/enemySoldier_AI/AIC_enemyBase_AIController.AIC_enemyBase_AIController_C|GetAttack%20Target _asaic_enemy_base_aicontroller)
            (:then
              (bind _returnvalue_2 (Collision|LineTraceByChannel _returnvalue (Transformation|GetActorLocation _attack_target) "TraceTypeQuery1" false 0 "ForDuration"))
              (if (not _returnvalue_2)
                (Development|PrintString "Player Hit")
                (bind (_outhit _returnvalue_3) (Collision|LineTraceByChannel _returnvalue (Transformation|GetActorLocation _attack_target) "TraceTypeQuery1" false 0 "None"))
                (if _returnvalue_3
                  (Class|BPIDamagable|ActorTakeDamage(Message) (.HitActor (Collision|BreakHitResult _outhit)) (Utilities|Struct|MakeS_DamageInfo 2e+02 "NewEnumerator3" "NewEnumerator1")))))
            (:else)))))))

(fn ConstructionScript
  (|CallParentFunction))

(fn GetIdealRange
  (return 3e+02 5e+02))

(fn GetActorCurrentHealth
  (return (Variables|/Game/DamageSystem/BPC_DamageSystem.BPC_DamageSystem_C|GetActorCurrentHealth (Variables|Default|GetBPC_DamageSystem))))

(fn ActorTakeDamage
  (params (DamageInfo :type S%20Damage%20Info%20Structure))
  (return false))

(fn GetActorMaxHealth
  (return (Variables|/Game/DamageSystem/BPC_DamageSystem.BPC_DamageSystem_C|GetActorMaxHealth (Variables|Default|GetBPC_DamageSystem))))

(fn HealActor
  (params (HealAmount :type Float%20%28double-precision%29))
  (bind _newhp (Default|HealActor (Variables|Default|GetBPC_DamageSystem) HealAmount))
  (return _newhp))