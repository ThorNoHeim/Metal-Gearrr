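; Melee enemy soldier Blueprint that equips a sword and performs a slash attack.
; EquipWeapon spawns BP_WeaponSword, snaps it to the mesh's RightHandGrip socket and flags the soldier as wielding a weapon.
; The generically named CustomEvent plays the sword slash montage and fires OnAttackEnd on completion or interruption, so listeners are notified either way.
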(event Custom|CustomEvent
  (Animation|Montage|PlayMontage (Variables|Character|GetMesh) "/Game/Characters/Enemies/Enemy_Soldier/enemySoldier_Animations/AM_swordSlash.AM_swordSlash"
    (:OnCompleted
      _)
    (:OnInterrupted
      _))
  (Default|CallOnAttackEnd))

(event EventBeginPlay
  (|CallParentFunction) ; This node is disabled and will not be called.\nDrag off pins to build functionality.
)

(event Collision|EventActorBeginOverlap
  (params (OtherActor :type Actor%20Object%20Reference)))

(event EventEquipWeapon
  (bind _returnvalue (Game|SpawnActorfromClass "/Game/Characters/Enemies/Enemy_Soldier/Weapons/BP_WeaponSword.BP_WeaponSword_C" (Transformation|GetActorTransform) "Undefined" "MultiplyWithRoot" 0 0))
  (Transformation|AttachComponentToComponent _returnvalue (Variables|Character|GetMesh) "RightHandGrip" "SnapToTarget" "SnapToTarget" "SnapToTarget" true)
  (Variables|Default|SetisWieldingWeapon true))

(event EventTick
  (params (DeltaSeconds :type Float%20%28single-precision%29)))

(fn ConstructionScript
  (|CallParentFunction))