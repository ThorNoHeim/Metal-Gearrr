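; BP_enemySoldierBase is the base soldier enemy character, exposing health, combat range, patrol and movement functions.
; Damage, healing and health queries are forwarded to its BPCDamageSystem component.
; It supplies fixed attack and circling radii along with its assigned patrol route.
; SetMovementSpeed maps named speed states from idle to sprint onto the CharacterMovement max walk speed.
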(fn ConstructionScript)

(fn ActorTakeDamage
  (params (DamageInfo :type S%20Damage%20Info%20Structure))
  (bind _wasdamaged (Default|ActorTakeDamage (Variables|Default|GetBPC_DamageSystem) DamageInfo))
  (return _wasdamaged))

(fn GetActorCurrentHealth
  (return (Variables|/Game/DamageSystem/BPC_DamageSystem.BPC_DamageSystem_C|GetActorCurrentHealth (Variables|Default|GetBPC_DamageSystem))))

(fn GetActorMaxHealth
  (return (Variables|/Game/DamageSystem/BPC_DamageSystem.BPC_DamageSystem_C|GetActorMaxHealth (Variables|Default|GetBPC_DamageSystem))))

(fn GetIdealRange
  (return 3e+02 4.5e+02))

(fn GetPatrolRoute
  (return (Variables|AI|GetPatrolRoute)))

(fn HealActor
  (params (HealAmount :type Float%20%28double-precision%29))
  (bind _newhp (Default|HealActor (Variables|Default|GetBPC_DamageSystem) HealAmount))
  (return _newhp))

(fn SetMovementSpeed
  (params (Speed :type E_MovementSpeed%20Enum :default "NewEnumerator0"))
  (bind _output_get (Variables|/Script/Engine.CharacterMovementComponent|SetMaxWalkSpeed (Variables|Character|GetCharacterMovement) (Utilities|Select :Index Speed :NewEnumerator0 0.0 :NewEnumerator1 2e+02 :NewEnumerator2 3.1e+02 :NewEnumerator3 4.5e+02 :NewEnumerator4 6e+02)))
  (return _output_get))