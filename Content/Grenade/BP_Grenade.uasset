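; BP_Grenade is a timed grenade actor that explodes three seconds after it begins play.
; On detonation it fires a RadialForce impulse and spawns a tutorial particle emitter at the Grenade component's location, then destroys itself after another delay.
; A downward sphere trace runs just before the blast, but nothing uses its hit results, and the graph applies no damage.
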(event Collision|EventActorBeginOverlap
  (params (OtherActor :type Actor%20Object%20Reference)))

(event EventTick
  (params (DeltaSeconds :type Float%20%28single-precision%29)))

(event EventBeginPlay
  (Utilities|FlowControl|Delay 3.0)
  (bind _output_get (Variables|Default|SetNewVar (Transformation|GetWorldLocation (Variables|Default|GetGrenade))))
  (bind _outhit (Collision|SphereTraceByChannel _output_get (- _output_get "0.000000,0.000000,50.000000") 3e+02 "TraceTypeQuery1" false 0 "None"))
  (Variables|Default|SetImpact%20Point (.ImpactPoint (Collision|BreakHitResult _outhit)))
  (Variables|Default|SetHit%20Actor (.HitActor (Collision|BreakHitResult _outhit)))
  (Class|RadialForceComponent|FireImpulse (Variables|Default|GetRadialForce))
  (Effects|SpawnEmitteratLocation "/Engine/Tutorial/SubEditors/TutorialAssets/TutorialParticleSystem.TutorialParticleSystem" (Transformation|GetWorldLocation (Variables|Default|GetGrenade)))
  (Utilities|FlowControl|Delay 3.0)
  (Actor|DestroyActor))

(fn ConstructionScript)